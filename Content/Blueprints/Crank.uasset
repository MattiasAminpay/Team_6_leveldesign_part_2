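; Crank interactable that the side-scroller character triggers with the Interact input while standing in its box.
; Box overlap swaps the text on Er and opens or closes a gate, with input enabled on begin overlap.
; An Interact press through the open gate sends InteractMessage(false) to Target and makes the crank's static mesh visible.
; Input is never disabled, so the gate alone limits interaction to the overlap.
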(event OnComponentBeginOverlap(Box)
  (params (OverlappedComponent :type Primitive%20Component%20Object%20Reference) (OtherActor :type Actor%20Object%20Reference) (OtherComp :type Primitive%20Component%20Object%20Reference) (OtherBodyIndex :type Integer) (bFromSweep :type Boolean) (SweepResult :type Hit%20Result%20Structure%20%28by%20ref%29))
  (Utilities|Casting|CastToSideScrollerCharacter_2 OtherActor)
  (Input|EnableInput (Game|GetPlayerController 0))
  (Rendering|Components|TextRender|SetText (Variables|Default|Geter) (Variables|Default|GetValue))
  (Utilities|FlowControl|Gate true) ; enters at Open
)

(event OnComponentEndOverlap(Box)
  (params (OverlappedComponent :type Primitive%20Component%20Object%20Reference) (OtherActor :type Actor%20Object%20Reference) (OtherComp :type Primitive%20Component%20Object%20Reference) (OtherBodyIndex :type Integer))
  (Utilities|Casting|CastToSideScrollerCharacter_2 OtherActor)
  (Rendering|Components|TextRender|SetText (Variables|Default|Geter) (Variables|Default|GetValue_0))
  (Utilities|FlowControl|Gate true) ; enters at Close
)

(event Input|ActionEvents|InputActionInteract
  (params (Key :type Key%20Structure :default "None"))
  (:Pressed
    (Utilities|FlowControl|Gate true
      (:Exit
        (Class|InteractInterface|Interact(Message) (Variables|Default|GetTarget) false)
        (Rendering|SetVisibility (Variables|Default|GetStaticMesh) true false)))))

(fn ConstructionScript)