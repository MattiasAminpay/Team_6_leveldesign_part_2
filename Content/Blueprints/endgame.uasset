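; Interactable end-of-game trigger that fades the screen to black and loads the "endgame" level.
; A box overlap by SideScrollerCharacter_2 enables input and opens a gate, which closes when the character leaves.
; Pressing Interact through the open gate plays a timeline that drives the manual camera fade.
; The timeline's update also starts a delay before the level opens.
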(event OnComponentBeginOverlap(Box)
  (params (OverlappedComponent :type Primitive%20Component%20Object%20Reference) (OtherActor :type Actor%20Object%20Reference) (OtherComp :type Primitive%20Component%20Object%20Reference) (OtherBodyIndex :type Integer) (bFromSweep :type Boolean) (SweepResult :type Hit%20Result%20Structure%20%28by%20ref%29))
  (Utilities|Casting|CastToSideScrollerCharacter_2 OtherActor)
  (Input|EnableInput (Game|GetPlayerController 0))
  (Utilities|FlowControl|Gate true) ; enters at Open
)

(event OnComponentEndOverlap(Box)
  (params (OverlappedComponent :type Primitive%20Component%20Object%20Reference) (OtherActor :type Actor%20Object%20Reference) (OtherComp :type Primitive%20Component%20Object%20Reference) (OtherBodyIndex :type Integer))
  (Utilities|Casting|CastToSideScrollerCharacter_2 OtherActor)
  (Utilities|FlowControl|Gate true) ; enters at Close
)

(event Input|ActionEvents|InputActionInteract
  (params (Key :type Key%20Structure :default "None"))
  (:Pressed
    (Utilities|FlowControl|Gate true
      (:Exit
        (bind _newtrack_0 (Timeline|Timeline_0 Play)
          (:Update
            (Class|PlayerCameraManager|SetManualCameraFade :self (Game|GetPlayerCameraManager 0) :InFadeAmount _newtrack_0)
            (Utilities|FlowControl|Delay 5.0)
            (Game|OpenLevel(byName) "endgame")))))))

(fn ConstructionScript)